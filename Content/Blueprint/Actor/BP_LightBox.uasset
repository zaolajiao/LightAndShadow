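; Pushable light box that lights up to five areas, adjusting the player's light counter and destroying enemies that enter them.
; The X and Y triggers enable cube physics and flag the character as pushing while overlapped.
; On BeginPlay and when a push overlap ends, line traces recompute how many consecutive areas are lit before an obstruction.
; A forward trace also makes the BP_SpecialBlock it hits passable, restoring the previous one's collision.
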(event `self.ReceiveBeginPlay`
  (`self.InitAreaArray`)
  (`self.RefreshBlock`)
  (`self.RefreshArea`))

(event `self.XCollision.OnComponentBeginOverlap`
  (params (OverlappedComponent :type "PrimitiveComponent Object Reference") (OtherActor :type "Actor Object Reference") (OtherComp :type "PrimitiveComponent Object Reference") (OtherBodyIndex :type Integer) (bFromSweep :type Boolean) (SweepResult :type "HitResult Structure (by ref)"))
  ;[1 1 1] X collision
  (bind _asbp_third_person_character (cast `/Game/ThirdPerson/Blueprints/BP_ThirdPersonCharacter` OtherActor))
  (`PrimitiveComponent.SetSimulatePhysics` (`self.Cube`) true)
  (set `/Game/ThirdPerson/Blueprints/BP_ThirdPersonCharacter.IsPushing` true _asbp_third_person_character)
  (set `/Game/ThirdPerson/Blueprints/BP_ThirdPersonCharacter.OverlapActor` self _asbp_third_person_character))

(event `self.XCollision.OnComponentEndOverlap`
  (params (OverlappedComponent :type "PrimitiveComponent Object Reference") (OtherActor :type "Actor Object Reference") (OtherComp :type "PrimitiveComponent Object Reference") (OtherBodyIndex :type Integer))
  ;[1 1 1] X collision
  (bind _asbp_third_person_character (cast `/Game/ThirdPerson/Blueprints/BP_ThirdPersonCharacter` OtherActor))
  (`PrimitiveComponent.SetSimulatePhysics` (`self.Cube`) false)
  (`self.RefreshBlock`)
  (`self.RefreshArea`)
  (set `/Game/ThirdPerson/Blueprints/BP_ThirdPersonCharacter.IsPushing` false _asbp_third_person_character)
  (set `/Game/ThirdPerson/Blueprints/BP_ThirdPersonCharacter.OverlapActor` null _asbp_third_person_character))

(event `self.YCollision.OnComponentBeginOverlap`
  (params (OverlappedComponent :type "PrimitiveComponent Object Reference") (OtherActor :type "Actor Object Reference") (OtherComp :type "PrimitiveComponent Object Reference") (OtherBodyIndex :type Integer) (bFromSweep :type Boolean) (SweepResult :type "HitResult Structure (by ref)"))
  ;[1 1 1] Y collision
  (bind _asbp_third_person_character (cast `/Game/ThirdPerson/Blueprints/BP_ThirdPersonCharacter` OtherActor))
  (`PrimitiveComponent.SetSimulatePhysics` (`self.Cube`) true)
  (set `/Game/ThirdPerson/Blueprints/BP_ThirdPersonCharacter.IsPushing` true _asbp_third_person_character)
  (set `/Game/ThirdPerson/Blueprints/BP_ThirdPersonCharacter.OverlapActor` self _asbp_third_person_character))

(event `self.YCollision.OnComponentEndOverlap`
  (params (OverlappedComponent :type "PrimitiveComponent Object Reference") (OtherActor :type "Actor Object Reference") (OtherComp :type "PrimitiveComponent Object Reference") (OtherBodyIndex :type Integer))
  ;[1 1 1] Y collision
  (bind _asbp_third_person_character (cast `/Game/ThirdPerson/Blueprints/BP_ThirdPersonCharacter` OtherActor))
  (`PrimitiveComponent.SetSimulatePhysics` (`self.Cube`) false)
  (`self.RefreshBlock`)
  (`self.RefreshArea`)
  (set `/Game/ThirdPerson/Blueprints/BP_ThirdPersonCharacter.IsPushing` false _asbp_third_person_character)
  (set `/Game/ThirdPerson/Blueprints/BP_ThirdPersonCharacter.OverlapActor` null _asbp_third_person_character))

(event `self.Area0.OnComponentBeginOverlap`
  (params (OverlappedComponent :type "PrimitiveComponent Object Reference") (OtherActor :type "Actor Object Reference") (OtherComp :type "PrimitiveComponent Object Reference") (OtherBodyIndex :type Integer) (bFromSweep :type Boolean) (SweepResult :type "HitResult Structure (by ref)"))
  ;[1 1 1] Area Overlap
  (`self.BeginOverlapActor` OtherActor))

(event `self.Area0.OnComponentEndOverlap`
  (params (OverlappedComponent :type "PrimitiveComponent Object Reference") (OtherActor :type "Actor Object Reference") (OtherComp :type "PrimitiveComponent Object Reference") (OtherBodyIndex :type Integer))
  ;[1 1 1] Area Overlap
  (`self.EndOverlapActor` OtherActor))

(event `self.Area1.OnComponentBeginOverlap`
  (params (OverlappedComponent :type "PrimitiveComponent Object Reference") (OtherActor :type "Actor Object Reference") (OtherComp :type "PrimitiveComponent Object Reference") (OtherBodyIndex :type Integer) (bFromSweep :type Boolean) (SweepResult :type "HitResult Structure (by ref)"))
  ;[1 1 1] Area Overlap
  (if (>= (`self.LitAreaLevel`) 1)
    (`self.BeginOverlapActor` OtherActor)))

(event `self.Area1.OnComponentEndOverlap`
  (params (OverlappedComponent :type "PrimitiveComponent Object Reference") (OtherActor :type "Actor Object Reference") (OtherComp :type "PrimitiveComponent Object Reference") (OtherBodyIndex :type Integer))
  ;[1 1 1] Area Overlap
  (if (>= (`self.LitAreaLevel`) 1)
    (`self.EndOverlapActor` OtherActor)))

(event `self.Area2.OnComponentBeginOverlap`
  (params (OverlappedComponent :type "PrimitiveComponent Object Reference") (OtherActor :type "Actor Object Reference") (OtherComp :type "PrimitiveComponent Object Reference") (OtherBodyIndex :type Integer) (bFromSweep :type Boolean) (SweepResult :type "HitResult Structure (by ref)"))
  ;[1 1 1] Area Overlap
  (if (>= (`self.LitAreaLevel`) 2)
    (`self.BeginOverlapActor` OtherActor)))

(event `self.Area2.OnComponentEndOverlap`
  (params (OverlappedComponent :type "PrimitiveComponent Object Reference") (OtherActor :type "Actor Object Reference") (OtherComp :type "PrimitiveComponent Object Reference") (OtherBodyIndex :type Integer))
  ;[1 1 1] Area Overlap
  (if (>= (`self.LitAreaLevel`) 2)
    (`self.EndOverlapActor` OtherActor)))

(event `self.Area3.OnComponentBeginOverlap`
  (params (OverlappedComponent :type "PrimitiveComponent Object Reference") (OtherActor :type "Actor Object Reference") (OtherComp :type "PrimitiveComponent Object Reference") (OtherBodyIndex :type Integer) (bFromSweep :type Boolean) (SweepResult :type "HitResult Structure (by ref)"))
  ;[1 1 1] Area Overlap
  (if (>= (`self.LitAreaLevel`) 3)
    (`self.BeginOverlapActor` OtherActor)))

(event `self.Area3.OnComponentEndOverlap`
  (params (OverlappedComponent :type "PrimitiveComponent Object Reference") (OtherActor :type "Actor Object Reference") (OtherComp :type "PrimitiveComponent Object Reference") (OtherBodyIndex :type Integer))
  ;[1 1 1] Area Overlap
  (if (>= (`self.LitAreaLevel`) 3)
    (`self.EndOverlapActor` OtherActor)))

(event `self.Area4.OnComponentBeginOverlap`
  (params (OverlappedComponent :type "PrimitiveComponent Object Reference") (OtherActor :type "Actor Object Reference") (OtherComp :type "PrimitiveComponent Object Reference") (OtherBodyIndex :type Integer) (bFromSweep :type Boolean) (SweepResult :type "HitResult Structure (by ref)"))
  ;[1 1 1] Area Overlap
  (if (>= (`self.LitAreaLevel`) 4)
    (`self.BeginOverlapActor` OtherActor)))

(event `self.Area4.OnComponentEndOverlap`
  (params (OverlappedComponent :type "PrimitiveComponent Object Reference") (OtherActor :type "Actor Object Reference") (OtherComp :type "PrimitiveComponent Object Reference") (OtherBodyIndex :type Integer))
  ;[1 1 1] Area Overlap
  (if (>= (`self.LitAreaLevel`) 4)
    (`self.EndOverlapActor` OtherActor)))

(fn `BeginOverlapActor`
  (params (actor :type "Actor Object Reference"))
  (bind _asbp_third_person_character (cast `/Game/ThirdPerson/Blueprints/BP_ThirdPersonCharacter` actor)
    (:`then`
      (`LightAndShadowCharacter.AddLightCounter` _asbp_third_person_character))
    (:`CastFailed`
      (bind _asbp_enemy_character (cast `/Game/Blueprint/Actor/BP_EnemyCharacter` actor))
      (`GameplayStatics.SpawnEmitterAtLocation` "/Game/Particles/P_Destruction_Metal.P_Destruction_Metal" (`self.K2_GetActorLocation` _asbp_enemy_character))
      (`self.K2_DestroyActor` _asbp_enemy_character))))

(fn `EndOverlapActor`
  (params (actor :type "Actor Object Reference"))
  (bind _asbp_third_person_character (cast `/Game/ThirdPerson/Blueprints/BP_ThirdPersonCharacter` actor))
  (`LightAndShadowCharacter.DecLightCounter` _asbp_third_person_character))

(fn `InitAreaArray`
  (set `self.AreaCollision` (`|MakeArray` (`self.Area0`) (`self.Area1`) (`self.Area2`) (`self.Area3`) (`self.Area4`))))

(fn `RefreshArea`
  (set `self.LitAreaLevel` 0)
  (for (_array_element _array_index) (`self.AreaCollision`)
    (if (== _array_index (`KismetArrayLibrary.Array_Length` (`self.AreaCollision`)))
      (break)
      (else
        (bind _returnvalue (`SceneComponent.K2_GetComponentLocation` _array_element))
        (bind _returnvalue_2 (* (`SceneComponent.GetForwardVector` _array_element) (80.0 80.0 80.0)))
        (bind _outhit (`KismetSystemLibrary.LineTraceSingle` (- _returnvalue _returnvalue_2) (+ _returnvalue _returnvalue_2) "TraceTypeQuery1"))
        (bind (_bblockinghit _binitialoverlap _time _distance _location _impactpoint _normal _impactnormal _physmat _hitactor) (`GameplayStatics.BreakHitResult` _outhit))
        (cast `/Game/Blueprint/Actor/BP_LightBox` _hitactor
          (:`then`
            _)
          (:`CastFailed`
            (if (== _hitactor null)
              _
              (else
                (break)))))
        (bind _result (`/Engine/EditorBlueprintResources/StandardMacros.IncrementInt` (`self.LitAreaLevel`))
          (:`  `
            (set `self.LitAreaLevel` _result)))))))

(fn `RefreshBlock`
  (bind _cube (`self.Cube`))
  (bind _returnvalue (`SceneComponent.K2_GetComponentLocation` _cube))
  (bind _asbp_special_block (cast `/Game/Blueprint/Actor/BP_SpecialBlock` (`self.Hit Actor`))
    (:`then`
      (`self.SetActorEnableCollision` _asbp_special_block true)
      (`PrimitiveComponent.SetCollisionEnabled` (`/Game/Blueprint/Actor/BP_SpecialBlock.Cube` _asbp_special_block) "QueryAndPhysics")
      (`PrimitiveComponent.SetCollisionResponseToAllChannels` (`/Game/Blueprint/Actor/BP_SpecialBlock.Cube` _asbp_special_block) "ECR_Block"))
    (:`CastFailed`
      _))
  (set `self.Hit Actor` null)
  (bind _outhit (`KismetSystemLibrary.LineTraceSingle` _returnvalue (+ _returnvalue (* (`SceneComponent.GetForwardVector` _cube) (1000.0 1000.0 1000.0))) "TraceTypeQuery1"))
  (bind (_bblockinghit _binitialoverlap _time _distance _location _impactpoint _normal _impactnormal _physmat _hitactor) (`GameplayStatics.BreakHitResult` _outhit))
  (bind _asbp_special_block_2 (cast `/Game/Blueprint/Actor/BP_SpecialBlock` _hitactor))
  (bind _cube_2 (`/Game/Blueprint/Actor/BP_SpecialBlock.Cube` _asbp_special_block_2))
  (`PrimitiveComponent.SetCollisionEnabled` _cube_2 "QueryOnly")
  (`PrimitiveComponent.SetCollisionResponseToAllChannels` _cube_2 "ECR_Ignore")
  (set `self.Hit Actor` _hitactor))

(fn `UserConstructionScript`)