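; BP_Bookcase is an interactable bookcase actor that shows dialogue lines to the player.
; On overlap it registers itself as the third-person character's OverlapActor and shows an animated confirm icon, undoing both when overlap ends.
; Each Talk call shows the next Dialogue entry in a lazily created dialog widget, returning false until the lines run out, then removes the widget, resets the index and returns true.
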(event `self.ReceiveActorBeginOverlap`
  (params (OtherActor :type "Actor Object Reference"))
  (bind _asbp_third_person_character (cast `/Game/ThirdPerson/Blueprints/BP_ThirdPersonCharacter` OtherActor))
  (set `/Game/ThirdPerson/Blueprints/BP_ThirdPersonCharacter.OverlapActor` self _asbp_third_person_character)
  (`SceneComponent.SetVisibility` (`self.TalkIcon`) true false)
  (bind _asbp_confirm_icon_widget (cast `/Game/Blueprint/Widget/BP_ConfirmIconWidget` (`WidgetComponent.GetWidget` (`self.TalkIcon`))))
  (`/Game/Blueprint/Widget/BP_ConfirmIconWidget.StartAnimation` _asbp_confirm_icon_widget))

(event `self.ReceiveActorEndOverlap`
  (params (OtherActor :type "Actor Object Reference"))
  (bind _asbp_third_person_character (cast `/Game/ThirdPerson/Blueprints/BP_ThirdPersonCharacter` OtherActor))
  (set `/Game/ThirdPerson/Blueprints/BP_ThirdPersonCharacter.OverlapActor` null _asbp_third_person_character)
  (`SceneComponent.SetVisibility` (`self.TalkIcon`) false false)
  (bind _asbp_confirm_icon_widget (cast `/Game/Blueprint/Widget/BP_ConfirmIconWidget` (`WidgetComponent.GetWidget` (`self.TalkIcon`))))
  (`/Game/Blueprint/Widget/BP_ConfirmIconWidget.FinishAnimation` _asbp_confirm_icon_widget))

(fn `Talk`
  (returns (finish :type Boolean))
  (if (< (`self.TalkIndex`) (`KismetArrayLibrary.Array_Length` (`self.Dialogue`)))
    (`/Engine/EditorBlueprintResources/StandardMacros.IsValid` (`self.DialogWidget`)
      (:`Is Valid`
        _)
      (:`Is Not Valid`
        (bind _returnvalue (`|CreateWidget` "/Game/Blueprint/Widget/BP_DialogWidget.BP_DialogWidget_C"))
        (`UserWidget.AddToViewport` _returnvalue 0)
        (set `self.DialogWidget` _returnvalue)))
    (`TextBlock.SetText` (`/Game/Blueprint/Widget/BP_DialogWidget.TalkText` (`self.DialogWidget`)) (`KismetTextLibrary.Conv_StringToText` (`|GetArrayItem` (`self.Dialogue`) (`self.TalkIndex`))))
    (`/Engine/EditorBlueprintResources/StandardMacros.IncrementInt` (`self.TalkIndex`)
      (:`  `
        (return false)))
    (else
      (`Widget.RemoveFromParent` (`self.DialogWidget`))
      (set `self.DialogWidget` null)
      (set `self.TalkIndex` 0)
      (return true))))

(fn `UserConstructionScript`)