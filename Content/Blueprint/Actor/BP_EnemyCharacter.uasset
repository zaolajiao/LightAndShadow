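; BP_EnemyCharacter is an enemy character that chases the player and deals melee-style damage on reaching them.
; From BeginPlay, a self-calling custom event issues AI MoveTo toward the player's current location, re-issuing it after a short delay without waiting for completion.
; A successful move plays the attack montage, then applies damage to the player after a fixed delay, with no further range check.
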(event `self.ReceiveBeginPlay`
  (`self.CustomEvent`))

(event `self.ReceiveTick`
  (params (DeltaSeconds :type "Float (single-precision)")))

(event `CustomEvent`
  (`|AIMoveTo` self (`self.K2_GetActorLocation` (`GameplayStatics.GetPlayerCharacter` 0)) null 10.0
    (:`then`
      (`KismetSystemLibrary.Delay` 1.0)
      (`self.CustomEvent`))
    (:`OnSuccess`
      (`self.PlayAnimMontage` "/Game/Animations/AnimationMontage/AttackMontage.AttackMontage")
      (`KismetSystemLibrary.Delay` 1.0)
      (`GameplayStatics.ApplyDamage` (`GameplayStatics.GetPlayerCharacter` 0) 1.0 (`self.GetController` self) self "/Script/Engine.DamageType"))))

(fn `UserConstructionScript`)